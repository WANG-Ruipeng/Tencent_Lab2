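; BP_Target is a shootable target actor that bobs vertically and awards score when damaged.
; Every tick, MoveOnServer offsets the mesh along Z by a sine of clock seconds, stores CurrentLocation, then calls MoveOnClient to apply it.
; Damage increments the instigator's MyPlayerState score, and the actor is destroyed only when that cast fails.
; CurrentLocation has a RepNotify, but its handler is empty.
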(event `self.ReceiveTick`
  (params (DeltaSeconds :type "Float (single-precision)"))
  (`self.MoveOnServer`))

(event `MoveOnServer`
  ;[1 1 1] Server Refresh Position
  (`SceneComponent.K2_AddLocalOffset` (`self.Target`) (`KismetMathLibrary.MakeVector` 0.0 0.0 (`KismetMathLibrary.Sin` (* (`.Second` (`KismetMathLibrary.BreakDateTime` (`KismetMathLibrary.Now`))) 1.5))) false false)
  (set `self.CurrentLocation` (`SceneComponent.K2_GetComponentLocation` (`self.Target`)))
  (`self.MoveOnClient`))

(event `MoveOnClient`
  ;[1 1 1] Refresh Position Locally
  (`SceneComponent.K2_SetWorldLocation` (`self.Target`) (`self.CurrentLocation`) false false))

(event `self.ReceiveAnyDamage`
  (params (Damage :type "Float (single-precision)") (DamageType :type "DamageType Object Reference") (InstigatedBy :type "Controller Object Reference") (DamageCauser :type "Actor Object Reference"))
  (bind _asmy_player_state (cast `/Game/Blueprints/MyPlayerState` (`Controller.PlayerState` InstigatedBy))
    (:`then`
      (`/Game/Blueprints/MyPlayerState.IncrementScore` _asmy_player_state))
    (:`CastFailed`
      (`self.K2_DestroyActor`))))

(fn `OnRep_CurrentLocation`)

(fn `UserConstructionScript`)